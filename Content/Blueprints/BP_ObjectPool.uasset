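; BP_ObjectPool is an actor that pre-spawns and pools BP_TankShell projectiles for reuse.
; On BeginPlay it spawns shells at the world origin, owned by the pool, in a loop bounded by ObjectsToSpawn and stores them in an array.
; GetTankShell pops the last shell from the array and hands it out.
; The file has no return-to-pool logic and no empty-array check.
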(event `self.ReceiveBeginPlay`
  (for _ (range (+ (`self.ObjectsToSpawn`) 1))
    (bind _returnvalue (`|SpawnActorFromClass` "/Game/Blueprints/BP_TankShell.BP_TankShell_C" (`KismetMathLibrary.MakeTransform` (0.0 0.0 0.0)) "Undefined" "MultiplyWithRoot" self null))
    (`KismetArrayLibrary.Array_Add` (`self.BP_TankShell`) _returnvalue)))

(fn `Get Tank Shell`
  (returns (NewLocalVar1 :type "/Game/Blueprints/BP_TankShell Object Reference"))
  (locals (NewLocalVar :type "/Game/Blueprints/BP_TankShell Object Reference"))
  (bind _bp_tankshell (`self.BP_TankShell`))
  (bind _returnvalue (`KismetArrayLibrary.Array_LastIndex` _bp_tankshell))
  (set `local.NewLocalVar` (`|GetArrayItem` _bp_tankshell _returnvalue))
  (`KismetArrayLibrary.Array_Remove` _bp_tankshell _returnvalue)
  (return (`local.NewLocalVar`)))

(fn `UserConstructionScript`)