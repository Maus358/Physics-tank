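; Player-controlled tank pawn with physics-driven movement, an aimable turret and gun, and shell firing.
; Enhanced Input applies torque to six wheels, turning by opposing sides when stationary or driving one side when moving.
; Mouse input rotates the view, with turret yaw and clamped barrel pitch derived from camera look-at rotations.
; A left-mouse debug key activates shells from BP_ObjectPool at the barrel; the five-second cooldown logic is unconnected.
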(event Input|EnhancedActionEvents|EnhancedInputActionIA-Accelerate
  (params (ActionValue :type Float%20%28double-precision%29) (ElapsedSeconds :type Float%20%28double-precision%29) (TriggeredSeconds :type Float%20%28double-precision%29) (InputAction :type Input%20Action%20Object%20Reference :default "/Game/Blueprints/IA-Accelerate.IA-Accelerate"))
  (:Triggered
    (Variables|Default|SetIsMoving true :!label _label)
    (CallFunction|Acceleration ActionValue (Variables|Default|GetAccelration) (Variables|Default|GetFL_Wheel) (Variables|Default|GetML_Wheel) (Variables|Default|GetBL_Wheel) (Variables|Default|GetFR_Wheel) (Variables|Default|GetMR_Wheel) (Variables|Default|GetBR_Wheel)))
  (:Started
    (goto _label))
  (:Ongoing
    (goto _label))
  (:Canceled
    (Variables|Default|SetIsMoving false :!label _label_2))
  (:Completed
    (goto _label_2)))

(event Input|EnhancedActionEvents|EnhancedInputActionIA_Turn
  (params (ActionValue :type Float%20%28double-precision%29) (ElapsedSeconds :type Float%20%28double-precision%29) (TriggeredSeconds :type Float%20%28double-precision%29) (InputAction :type Input%20Action%20Object%20Reference :default "/Game/Blueprints/IA_Turn.IA_Turn"))
  (bind _accelration (Variables|Default|GetAccelration))
  (if (Variables|Default|GetIsMoving)
    (if (== ActionValue 1.0)
      (CallFunction|TruningontheMove 1.0 _accelration (Variables|Default|GetFL_Wheel) (Variables|Default|GetML_Wheel) (Variables|Default|GetBL_Wheel))
      (else
        (CallFunction|TruningontheMove 1.0 _accelration (Variables|Default|GetFR_Wheel) (Variables|Default|GetMR_Wheel) (Variables|Default|GetBR_Wheel))))
    (else
      (CallFunction|Turning (Variables|Default|GetFL_Wheel) (Variables|Default|GetML_Wheel) (Variables|Default|GetBL_Wheel) (Variables|Default|GetFR_Wheel) (Variables|Default|GetMR_Wheel) (Variables|Default|GetBR_Wheel) ActionValue (Variables|Default|GetTurning%20Speed)))))

(event EventBeginPlay
  (bind _returnvalue (Game|GetPlayerCameraManager 0))
  (Utilities|FlowControl|Sequence
    (:then_0
      (Input|AddMappingContext (PlayerController|LocalPlayerSubsystems|GetEnhancedInputLocalPlayerSubsystem (Game|GetPlayerController 0)) "/Game/Blueprints/IMC_TankMovement.IMC_TankMovement" 0 "(bIgnoreAllPressedKeysUntilRelease=True,bForceImmediately=False,bNotifyUserSettings=False)"))
    (:then_1
      (Variables|/Script/Engine.PlayerCameraManager|SetViewPitchMin _returnvalue -2e+01)
      (Variables|/Script/Engine.PlayerCameraManager|SetViewRollMax _returnvalue 15.0)
      (Variables|/Script/Engine.PlayerCameraManager|SetViewPitchMax _returnvalue 2e+01))
    (:then_2
      (bind _returnvalue_2 (Actor|GetActorOfClass "/Game/Blueprints/BP_ObjectPool.BP_ObjectPool_C"))
      (Variables|Default|SetBulletPool _returnvalue_2))))

(event Input|MouseEvents|MouseX
  (params (AxisValue :type Float%20%28single-precision%29))
  (Pawn|Input|AddControllerYawInput AxisValue)
  (CallFunction|TurretRotation AxisValue))

(event Input|MouseEvents|MouseY
  (params (AxisValue :type Float%20%28single-precision%29))
  (Pawn|Input|AddControllerPitchInput AxisValue)
  (CallFunction|GunElevation))

(event Input|MouseEvents|DebugKeyLeftMouseButton
  (params (Key :type Key%20Structure :default "None") (ActionValue :type Input%20Action%20Value%20Structure))
  (bind _barrel (Variables|Default|GetBarrel))
  (bind _str_tankshell_info (Variables|Default|GetSTR_TankShell_Info))
  (bind (_damage _speed _gravity) (Utilities|Struct|BreakSTR_TankShell_Info _str_tankshell_info))
  (:Pressed
    (bind _newlocalvar1 (Default|GetTankShell (Variables|Default|GetBulletPool)))
    (Default|Activate _newlocalvar1 (Utilities|Struct|MakeSTR_TankShell_Info (+ (Transformation|GetWorldLocation _barrel) (* (Math|Vector|GetForwardVector _barrel) 1e+02)) (Transformation|GetWorldRotation (Variables|Default|GetTurret)) _damage _speed "/Engine/EngineMeshes/Cube.Cube" _gravity))))

(fn ConstructionScript)

(fn TurretRotation
  (params (Axis%20Value :type Float%20%28double-precision%29))
  (bind _turret (Variables|Default|GetTurret))
  (Transformation|SetWorldRotation _turret (Math|Rotator|MakeRotator 0.0 0.0 (.yaw (Math|Rotator|FindLookatRotation (Transformation|GetWorldLocation (Variables|Default|GetCamera)) (Transformation|GetWorldLocation _turret)))) false false))

(fn Turning
  (params (FLW :type Static%20Mesh%20Component%20Object%20Reference) (MLW :type Static%20Mesh%20Component%20Object%20Reference) (BLW :type Static%20Mesh%20Component%20Object%20Reference) (FRW :type Static%20Mesh%20Component%20Object%20Reference) (MRW :type Static%20Mesh%20Component%20Object%20Reference) (BRW :type Static%20Mesh%20Component%20Object%20Reference) (InputValue :type Float%20%28double-precision%29) (Force :type Float%20%28double-precision%29))
  (Class|PrimitiveComponent|AddTorqueinDegrees FLW (Math|Vector|RotateVector (Math|Vector|MakeVector 0.0 (* InputValue Force) 0.0) (Transformation|GetWorldRotation (Variables|Default|GetBody))) "None" true)
  (Class|PrimitiveComponent|AddTorqueinDegrees BRW (Math|Vector|RotateVector (Math|Vector|MakeVector 0.0 (* InputValue Force -1.0) 0.0) (Transformation|GetWorldRotation (Variables|Default|GetBody))) "None" true))

(fn Acceleration
  (params (Input%20Value :type Float%20%28double-precision%29) (Force :type Float%20%28double-precision%29) (FLW :type Static%20Mesh%20Component%20Object%20Reference) (MLW :type Static%20Mesh%20Component%20Object%20Reference) (BLW :type Static%20Mesh%20Component%20Object%20Reference) (FRW :type Static%20Mesh%20Component%20Object%20Reference) (MRW :type Static%20Mesh%20Component%20Object%20Reference) (BRW :type Static%20Mesh%20Component%20Object%20Reference))
  (Class|PrimitiveComponent|AddTorqueinDegrees FLW (Math|Vector|RotateVector (Math|Vector|MakeVector 0.0 (* Input%20Value Force) 0.0) (Transformation|GetWorldRotation (Variables|Default|GetBody))) "None" true))

(fn TruningontheMove
  (params (Input%20Value :type Float%20%28double-precision%29) (Force :type Float%20%28double-precision%29) (FW :type Static%20Mesh%20Component%20Object%20Reference) (MW :type Static%20Mesh%20Component%20Object%20Reference) (BW :type Static%20Mesh%20Component%20Object%20Reference))
  (Class|PrimitiveComponent|AddTorqueinDegrees FW (Math|Vector|RotateVector (Math|Vector|MakeVector 0.0 (* Input%20Value Force) 0.0) (Transformation|GetWorldRotation (Variables|Default|GetBody))) "None" true))

(fn GunElevation
  (bind _barrel (Variables|Default|GetBarrel))
  (Transformation|SetRelativeRotation _barrel (Math|Rotator|MakeRotator 0.0 (Math|Float|Clamp(Float) (.pitch (Math|Rotator|FindLookatRotation (Transformation|GetWorldLocation (Variables|Default|GetCamera)) (Transformation|GetWorldLocation _barrel))) -8.0 1e+01) 0.0) false false))