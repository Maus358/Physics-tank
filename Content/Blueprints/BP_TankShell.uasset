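; Pooled tank shell projectile that is reused through BP_ObjectPool.
; Activate teleports it to the given transform, shows it, enables collision and applies the passed damage, speed, mesh and gravity.
; Any actor overlap triggers Deactivate, which hides it, disables collision and gravity, and adds it back to the owning pool's shell array.
; Damage is only stored here, and velocity is not reset on deactivation.
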(event `self.ReceiveBeginPlay`
  (`self.SetActorEnableCollision` false))

(event `Activate`
  (params (NewParam :type "/Game/Blueprints/STR_TankShell_Info Structure"))
  (bind (_position _rotation _damage _speed _mesh _gravity) (break `/Game/Blueprints/STR_TankShell_Info` NewParam))
  (bind _projectilemovement (`self.ProjectileMovement`))
  (`self.K2_SetActorLocationAndRotation` _position _rotation true true)
  (`self.SetActorHiddenInGame` false)
  (`self.SetActorEnableCollision` true)
  (set `self.Damage` _damage)
  (set `MovementComponent.Velocity` (* (`self.GetActorForwardVector`) _speed) _projectilemovement)
  (`StaticMeshComponent.SetStaticMesh` (`self.Sphere`) _mesh)
  (set `ProjectileMovementComponent.ProjectileGravityScale` _gravity _projectilemovement))

(event `Deactivate`
  (`self.SetActorHiddenInGame` true)
  (`self.SetActorEnableCollision` false)
  (set `ProjectileMovementComponent.ProjectileGravityScale` 0.0 (`self.ProjectileMovement`))
  (bind _asbp_object_pool (cast `/Game/Blueprints/BP_ObjectPool` (`self.GetOwner`)))
  (`KismetArrayLibrary.Array_Add` (`/Game/Blueprints/BP_ObjectPool.BP_TankShell` _asbp_object_pool) self))

(event `self.ReceiveActorBeginOverlap`
  (params (OtherActor :type "Actor Object Reference"))
  (`self.Deactivate`))

(fn `UserConstructionScript`)